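; BP_WalkingMachine is a pawn that stays idle until a BP_ZappingMachine damages it, then walks forward indefinitely.
; Damage from a zapping machine sets an IsOnline flag, which nothing in the file clears.
; While online, every Tick issues an AI MoveTo toward a point a short distance along its current forward vector, producing continuous straight-ahead movement.
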(event EventTick
  (params (DeltaSeconds :type Float%20%28single-precision%29))
  (if (Variables|Default|GetIsOnline?)
    (AI|AIMoveTo self (+ (Transformation|GetActorLocation) (* (Transformation|GetActorForwardVector) 2e+01)) 0 5.0 false)))

(event Game|Damage|EventAnyDamage
  (params (Damage :type Float%20%28single-precision%29) (DamageType :type Damage%20Type%20Object%20Reference) (InstigatedBy :type Controller%20Object%20Reference) (DamageCauser :type Actor%20Object%20Reference))
  (Utilities|Casting|CastToBP_ZappingMachine DamageCauser)
  (Variables|Default|SetIsOnline? true))

(fn ConstructionScript)