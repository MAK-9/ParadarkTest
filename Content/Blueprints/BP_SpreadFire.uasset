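; Short-lived fire-spreading actor that spawns BP_Fire on nearby flammable ground, then destroys itself.
; Shortly after BeginPlay it checks evenly spaced directions around itself, skipping any where a dot-product test finds an overlapping BP_Fire.
; For the rest, it traces down at a distance scaled from its Box extent and spawns fire where the hit surface type is Flammable or Burnable.
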(event Custom|End%20Fire
  (Actor|DestroyActor))

(event EventBeginPlay
  (Utilities|FlowControl|Sequence
    (:then_0
      (Utilities|FlowControl|Delay 0.1)
      (CallFunction|TrytoSpawnFire))
    (:then_1
      (Utilities|Time|SetTimerbyEvent (delegate Custom|End%20Fire) 0.2))))

(fn ConstructionScript)

(fn IsSurfaceFlammable
  (params (At :type Vector))
  (bind (_outhit _returnvalue) (Collision|LineTraceForObjects At (+ At "0, 0,-200.000000") (Utilities|Array|MakeArray "ObjectTypeQuery1") false 0 "None"))
  (if _returnvalue
    (switch Utilities|FlowControl|Switch|SwitchonEPhysicalSurface (Collision|GetSurfaceType _outhit)
      (:SurfaceType_Default
        (return false (.Location (Collision|BreakHitResult _outhit))))
      (:SurfaceType1
        _)
      (:SurfaceType3
        _))
    (return true (.Location (Collision|BreakHitResult _outhit)))))

(fn IsAlreadyBurning
  (params (Direction :type Vector))
  (for _array_element (Collision|GetOverlappingActors "/Game/Blueprints/BP_Fire.BP_Fire_C" :!class /Script/Engine.Actor)
    (if (>= (Math|Vector|DotProduct (- (Transformation|GetActorLocation _array_element) (Transformation|GetActorLocation)) Direction) 0.5)
      (return true)))
  (return false))

(fn TrytoSpawnFire
  (for _index (range 1 12)
    (bind _isburning (CallFunction|IsAlreadyBurning (Math|Vector|RotateVectorAroundAxis "1.000000,0.000000, 0" (Math|Conversions|ToFloat(Integer) (* _index 30)) "0, 0,1.000000")))
    (if (not _isburning)
      (bind (_isflammable _surfacelocation) (CallFunction|IsSurfaceFlammable (+ (* (Math|Vector|RotateVectorAroundAxis "1.000000,0.000000, 0" (Math|Conversions|ToFloat(Integer) (* _index 30)) "0, 0,1.000000") (* (.X (Math|Vector|BreakVector (Variables|/Script/Engine.BoxComponent|GetBoxExtent (Variables|Default|GetBox)))) 8.0)) (+ (Transformation|GetActorLocation) "0, 0,50.000000"))))
      (if _isflammable
        (Game|SpawnActorfromClass "/Game/Blueprints/BP_Fire.BP_Fire_C" (Math|Conversions|ToTransform(Vector) _surfacelocation) "AlwaysSpawn" 0 0)))))