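; BP_ZappingMachine is an actor that becomes an electrical hazard when it takes damage.
; Any damage calls StartZapping, which activates its initially inactive particle system, spawns a BP_SpreadFire at its transform and starts a looping timer.
; Zap runs immediately and on each timer tick, applying radial ElectricDamage within ZapRadius, with a debug sphere and a print when damage lands.
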(event Custom|Start%20Zapping
  (Components|Activation|Activate (Variables|Default|GetParticleSystem) false)
  (Utilities|Time|SetTimerbyEvent (delegate Custom|Zap!) 1.0 true)
  (Game|SpawnActorfromClass "/Game/Blueprints/BP_SpreadFire.BP_SpreadFire_C" (Transformation|GetActorTransform) "AlwaysSpawn" 0 0)
  (CallFunction|Zap!))

(event Custom|Zap!
  (bind _returnvalue (Transformation|GetActorLocation))
  (bind _zapradius (Variables|Default|GetZapRadius))
  (bind _returnvalue_2 (Game|Damage|ApplyRadialDamage 3.0 _returnvalue _zapradius "/Game/Blueprints/DamageTypes/ElectricDamage.ElectricDamage_C" 0 self 0 false "ECC_Visibility"))
  (Rendering|Debug|DrawDebugSphere _returnvalue _zapradius 12 "(R=0.000000,G=0.499369,B=1.000000,A=1.000000)" 0.5 1.0)
  (Development|PrintString "radian damage done" _returnvalue_2))

(event EventBeginPlay
  (Components|Activation|Deactivate (Variables|Default|GetParticleSystem)))

(event Game|Damage|EventAnyDamage
  (params (Damage :type Float%20%28single-precision%29) (DamageType :type Damage%20Type%20Object%20Reference) (InstigatedBy :type Controller%20Object%20Reference) (DamageCauser :type Actor%20Object%20Reference))
  (CallFunction|StartZapping))

(fn ConstructionScript)