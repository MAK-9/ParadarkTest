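; BP_ExplosiveBarrel is a barrel actor that explodes by spawning a BP_Explosion at its location and destroying itself.
; Overlapping a BP_Fire detonates it immediately.
; Being hit by a burning BP_AIEnemy, or taking damage from a player or another BP_Explosion, detonates it after ExplosionDelay, allowing chain reactions.
; All triggers funnel into the shared InitiateExplosion function.
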(event OnComponentBeginOverlap(BarrelMesh)
  (params (OverlappedComponent :type Primitive%20Component%20Object%20Reference) (OtherActor :type Actor%20Object%20Reference) (OtherComp :type Primitive%20Component%20Object%20Reference) (OtherBodyIndex :type Integer) (bFromSweep :type Boolean) (SweepResult :type Hit%20Result%20Structure%20%28by%20ref%29))
  (Utilities|Casting|CastToBP_Fire OtherActor)
  (CallFunction|InitiateExplosion))

(event OnComponentHit(BarrelMesh)
  (params (HitComponent :type Primitive%20Component%20Object%20Reference) (OtherActor :type Actor%20Object%20Reference) (OtherComp :type Primitive%20Component%20Object%20Reference) (NormalImpulse :type Vector :default "0, 0, 0") (Hit :type Hit%20Result%20Structure%20%28by%20ref%29))
  (bind _asbp_aienemy (Utilities|Casting|CastToBP_AIEnemy OtherActor))
  (bind _isonfire (Default|GetIsonFire _asbp_aienemy))
  (if _isonfire
    (Utilities|FlowControl|Delay (Variables|Default|GetExplosionDelay))
    (CallFunction|InitiateExplosion)))

(event Game|Damage|EventAnyDamage
  (params (Damage :type Float%20%28single-precision%29) (DamageType :type Damage%20Type%20Object%20Reference) (InstigatedBy :type Controller%20Object%20Reference) (DamageCauser :type Actor%20Object%20Reference))
  (Utilities|Casting|CastToPlayerController InstigatedBy
    (:then
      _)
    (:CastFailed
      (Utilities|Casting|CastToBP_Explosion DamageCauser)))
  (Utilities|FlowControl|Delay (Variables|Default|GetExplosionDelay))
  (CallFunction|InitiateExplosion))

(fn ConstructionScript)

(fn InitiateExplosion
  (Game|SpawnActorfromClass "/Game/Blueprints/BP_Explosion.BP_Explosion_C" (Math|Conversions|ToTransform(Vector) (Transformation|GetActorLocation)) "AlwaysSpawn" 0 0)
  (Actor|DestroyActor))