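; BP_Explosion is an explosion actor that deals radial fire damage around its location when it begins play.
; BeginPlay applies the damage within Radius, spawns BP_SpreadFire at the same transform and briefly draws a debug sphere of that radius.
; An older-looking overlap chain for damaging enemies, detonating barrels, firing a force impulse and destroying the actor is disconnected, so it never runs.
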(event EventBeginPlay
  (bind _returnvalue (Transformation|GetActorLocation))
  (bind _radius (Variables|Default|GetRadius))
  (Game|Damage|ApplyRadialDamage 5e+01 _returnvalue _radius "/Game/Blueprints/DamageTypes/FireDamage.FireDamage_C" 0 self 0 false "ECC_Visibility")
  (Game|SpawnActorfromClass "/Game/Blueprints/BP_SpreadFire.BP_SpreadFire_C" (Transformation|GetActorTransform) "Undefined" 0 0)
  (Rendering|Debug|DrawDebugSphere _returnvalue _radius 12 "(R=1.000000,G=0.556642,B=0.000000,A=1.000000)" 1.0 1.0))

(fn ConstructionScript)