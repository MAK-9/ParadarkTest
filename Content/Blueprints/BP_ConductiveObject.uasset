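; BP_ConductiveObject is an actor that becomes electrified for one second when it takes ElectricDamage.
; Electrification activates its particle system and spawns BP_SpreadFire at its transform.
; Box overlaps maintain the target list and start a looping timer, which applies ElectricDamage to those actors while electrified, so conductive objects can chain.
; When conduction stops, the particles deactivate and the damage timer is cleared until another overlap begins.
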(event OnComponentBeginOverlap(Box)
  (params (OverlappedComponent :type Primitive%20Component%20Object%20Reference) (OtherActor :type Actor%20Object%20Reference) (OtherComp :type Primitive%20Component%20Object%20Reference) (OtherBodyIndex :type Integer) (bFromSweep :type Boolean) (SweepResult :type Hit%20Result%20Structure%20%28by%20ref%29))
  (Utilities|Array|AddUnique (Variables|Default|GetElectrifiedActors) OtherActor)
  (bind _returnvalue (Utilities|Time|SetTimerbyFunctionName 0 "Deal Damage" 0.5 true)))

(event OnComponentEndOverlap(Box)
  (params (OverlappedComponent :type Primitive%20Component%20Object%20Reference) (OtherActor :type Actor%20Object%20Reference) (OtherComp :type Primitive%20Component%20Object%20Reference) (OtherBodyIndex :type Integer))
  (Utilities|Array|RemoveItem (Variables|Default|GetElectrifiedActors) OtherActor))

(event Custom|ConductElectricity
  (Variables|Default|SetIsElectrified true)
  (Components|Activation|Activate (Variables|Default|GetParticleSystem) false)
  (Utilities|Time|SetTimerbyEvent (delegate Custom|StopConducting) 1.0)
  (Game|SpawnActorfromClass "/Game/Blueprints/BP_SpreadFire.BP_SpreadFire_C" (Transformation|GetActorTransform) "AlwaysSpawn" 0 0))

(event Custom|StopConducting
  (Variables|Default|SetIsElectrified false)
  (Components|Activation|Deactivate (Variables|Default|GetParticleSystem))
  (Utilities|Time|ClearandInvalidateTimerbyHandle (stale OnComponentBeginOverlap(Box) _returnvalue)))

(event EventBeginPlay
  (Components|Activation|Deactivate (Variables|Default|GetParticleSystem)))

(event Game|Damage|EventAnyDamage
  (params (Damage :type Float%20%28single-precision%29) (DamageType :type Damage%20Type%20Object%20Reference) (InstigatedBy :type Controller%20Object%20Reference) (DamageCauser :type Actor%20Object%20Reference))
  (Utilities|Casting|CastToElectricDamage DamageType)
  (CallFunction|ConductElectricity))

(fn ConstructionScript)

(fn DealDamage
  (bind _electrifiedactors (Variables|Default|GetElectrifiedActors))
  (if (> (Utilities|Array|Length _electrifiedactors) 0)
    (if (Variables|Default|GetIsElectrified)
      (for _array_element _electrifiedactors
        (Game|Damage|ApplyDamage _array_element 3.0 0 0 "/Game/Blueprints/DamageTypes/ElectricDamage.ElectricDamage_C")))))