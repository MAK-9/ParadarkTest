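; Enemy pawn that chases the player on sight, shows its HP as text and can catch fire.
; Overlapping BP_Fire starts a looping timer that drains HP, spawns fire on Flammable floor found by a downward trace, and deals radial fire damage nearby.
; Burning stops three seconds after leaving the fire.
; All damage routes through ModifyHP; at zero HP, Death detaches the controller and ragdolls the mesh without clearing the burn timer.
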(event OnSeePawn(PawnSensing)
  (params (Pawn :type Pawn%20Object%20Reference))
  (bind _asfirst_person_character (Utilities|Casting|CastToFirstPersonCharacter Pawn))
  (AI|AIMoveTo self "0, 0, 0" _asfirst_person_character 5.0 false))

(event OnComponentBeginOverlap(CapsuleComponent)
  (params (OverlappedComponent :type Primitive%20Component%20Object%20Reference) (OtherActor :type Actor%20Object%20Reference) (OtherComp :type Primitive%20Component%20Object%20Reference) (OtherBodyIndex :type Integer) (bFromSweep :type Boolean) (SweepResult :type Hit%20Result%20Structure%20%28by%20ref%29))
  ;[1 1 1] Burning logic
  (Utilities|Casting|CastToBP_Fire OtherActor)
  (CallFunction|SetSelfonFire))

(event OnComponentEndOverlap(CapsuleComponent)
  (params (OverlappedComponent :type Primitive%20Component%20Object%20Reference) (OtherActor :type Actor%20Object%20Reference) (OtherComp :type Primitive%20Component%20Object%20Reference) (OtherBodyIndex :type Integer))
  ;[1 1 1] Burning logic
  (Utilities|Casting|CastToBP_Fire OtherActor)
  (Utilities|FlowControl|Delay 3.0)
  (CallFunction|ExtinguishSelf))

(event Custom|Set%20Self%20On%20Fire
  ;[1 1 1] Burning logic
  (Components|Activation|Activate (Variables|Default|GetParticleSystem) false)
  (if (not (Variables|Default|GetIsOnFire))
    (bind _returnvalue (Utilities|Time|SetTimerbyFunctionName 0 "FireDamage" 0.2 true))
    (Variables|Default|SetIsOnFire true)))

(event Custom|Extinguish%20Self
  ;[1 1 1] Burning logic
  (Utilities|Time|ClearandInvalidateTimerbyHandle (stale Custom|Set%20Self%20On%20Fire _returnvalue))
  (Components|Activation|Deactivate (Variables|Default|GetParticleSystem))
  (Variables|Default|SetIsOnFire false))

(event EventBeginPlay
  ;[1 1 1] Set HP to Max and update HPText
  (bind _output_get (Variables|Default|SetHPCurrent (Variables|Default|GetHPMax)))
  (Rendering|Components|TextRender|SetText (Variables|Default|GetHPText) (Utilities|Text|ToText(Integer) _output_get))
  ;[1 1 1] Start with Fire Particle OFF
  (Components|Activation|Deactivate (Variables|Default|GetParticleSystem)))

(event EventTick
  (params (DeltaSeconds :type Float%20%28single-precision%29))
  ;[1 1 1] Setting Floor on Fire
)

(event Game|Damage|EventAnyDamage
  (params (Damage :type Float%20%28single-precision%29) (DamageType :type Damage%20Type%20Object%20Reference) (InstigatedBy :type Controller%20Object%20Reference) (DamageCauser :type Actor%20Object%20Reference))
  (CallFunction|ModifyHP (Math|Float|Truncate Damage)))

(fn ConstructionScript)

(fn FireDamage
  (CallFunction|ModifyHP (Math|Random|RandomIntegerinRange 1 3))
  (CallFunction|SetFlooronFire)
  (CallFunction|SetNearbyonFire))

(fn ModifyHP
  (params (Amount :type Integer))
  (if (not (Variables|Default|GetIsDead))
    (bind _output_get (Variables|Default|SetHPCurrent (- (Variables|Default|GetHPCurrent) Amount)))
    (Rendering|Components|TextRender|SetText (Variables|Default|GetHPText) (Utilities|Text|ToText(Integer) _output_get))
    (if (<= (Variables|Default|GetHPCurrent) 0)
      (CallFunction|Death))))

(fn SetFlooronFire
  (bind _returnvalue (Transformation|GetActorLocation))
  (bind _returnvalue_2 (- _returnvalue "0, 0,100.000000"))
  (bind _outhit (Collision|LineTraceByChannel _returnvalue _returnvalue_2 "TraceTypeQuery1" false 0 "None"))
  (switch Utilities|FlowControl|Switch|SwitchonEPhysicalSurface (Collision|GetSurfaceType _outhit)
    (:SurfaceType1
      (Game|SpawnActorfromClass "/Game/Blueprints/BP_Fire.BP_Fire_C" (Math|Conversions|ToTransform(Vector) _returnvalue_2) "Undefined" 0 0))))

(fn GetIsonFire
  (return (Variables|Default|GetIsOnFire)))

(fn Death
  (bind _mesh (Variables|Character|GetMesh))
  (Variables|Default|SetIsDead true)
  (Rendering|SetVisibility (Variables|Default|GetHPText) false false)
  (Collision|SetCollisionEnabled (Variables|Collision|GetCapsuleComponent) "NoCollision")
  (Class|Pawn|DetachfromControllerPendingDestroy)
  (Pawn|Components|CharacterMovement|DisableMovement (Variables|Character|GetCharacterMovement))
  (Collision|SetCollisionEnabled _mesh "QueryAndPhysics")
  (Class|SkeletalMeshComponent|SetAllBodiesSimulatePhysics _mesh true)
  (Class|SkeletalMeshComponent|SetAllBodiesPhysicsBlendWeight _mesh 1.0 false))

(fn SetNearbyonFire
  (bind _returnvalue (Transformation|GetActorLocation))
  (bind _fireradius (LocalVariables|GetFireRadius))
  (Game|Damage|ApplyRadialDamage 3.0 _returnvalue _fireradius "/Game/Blueprints/DamageTypes/FireDamage.FireDamage_C" (Utilities|Array|MakeArray self) 0 0 false "ECC_Visibility")
  (Rendering|Debug|DrawDebugSphere _returnvalue _fireradius 12 "(R=0.656250,G=0.000000,B=0.016933,A=1.000000)" 1.0 1.0))