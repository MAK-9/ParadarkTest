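; BP_WalkingMachine is a machine pawn that starts walking once electric damage powers it online.
; Any damage of the ElectricDamage type sets IsOnline, and no logic here turns it off again.
; While online, Tick issues AI MoveTo each frame to a point just ahead along its forward vector.
; A MachineStatus widget component shows the online state, refreshed at BeginPlay and on activation.
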(event EventBeginPlay
  (CallFunction|UpdateStatusText))

(event EventTick
  (params (DeltaSeconds :type Float%20%28single-precision%29))
  (if (Variables|Default|GetIsOnline?)
    (AI|AIMoveTo self (+ (Transformation|GetActorLocation) (* (Transformation|GetActorForwardVector) 2e+01)) 0 5.0 false)))

(event Game|Damage|EventAnyDamage
  (params (Damage :type Float%20%28single-precision%29) (DamageType :type Damage%20Type%20Object%20Reference) (InstigatedBy :type Controller%20Object%20Reference) (DamageCauser :type Actor%20Object%20Reference))
  (Utilities|Casting|CastToElectricDamage DamageType)
  (Variables|Default|SetIsOnline? true)
  (CallFunction|UpdateStatusText))

(fn ConstructionScript)

(fn UpdateStatusText
  (bind _asmachine_status_widget (Utilities|Casting|CastToMachineStatusWidget (UserInterface|GetUserWidgetObject (Variables|Default|GetMachineStatus))))
  (Default|UpdateStatusText _asmachine_status_widget (Variables|Default|GetIsOnline?)))